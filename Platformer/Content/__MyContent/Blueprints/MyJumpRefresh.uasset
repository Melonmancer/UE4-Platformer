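; A jump refresh pickup volume that restores the player's double jump on contact.
; Box overlap events track whether the tagged player is inside; while true, Tick sets DoubleJump and fires EventJumpRefresh on the game manager's player.
; A Disappears flag makes it single-use, destroying the actor after refreshing.
; The construction script colors the cube red for disappearing instances and blue for persistent ones.
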(event OnComponentBeginOverlap(Box)
  (params (OverlappedComponent :type Primitive%20Component%20Object%20Reference) (OtherActor :type Actor%20Object%20Reference) (OtherComp :type Primitive%20Component%20Object%20Reference) (OtherBodyIndex :type Integer) (bFromSweep :type Boolean) (SweepResult :type Hit%20Result%20Structure%20%28by%20ref%29))
  (if (Actor|ActorHasTag OtherActor "Tag_Player")
    (Variables|Default|SetIs%20Overlapping true)))

(event OnComponentEndOverlap(Box)
  (params (OverlappedComponent :type Primitive%20Component%20Object%20Reference) (OtherActor :type Actor%20Object%20Reference) (OtherComp :type Primitive%20Component%20Object%20Reference) (OtherBodyIndex :type Integer))
  (if (Actor|ActorHasTag OtherActor "Tag_Player")
    (Variables|Default|SetIs%20Overlapping false)))

(event EventBeginPlay)

(event Collision|EventActorBeginOverlap
  (params (OtherActor :type Actor%20Object%20Reference)))

(event EventTick
  (params (DeltaSeconds :type Float%20%28single-precision%29))
  (if (Variables|Default|GetIs%20Overlapping)
    (bind _my_game_manager (CallFunction|GetMyGameManager))
    (Variables|/Game/ThirdPersonBP/Blueprints/ThirdPersonCharacter.ThirdPersonCharacter_C|SetDoubleJump (Variables|/Game/__MyContent/Blueprints/MyGameManager.MyGameManager_C|GetMyPlayer _my_game_manager) true)
    (Default|EventJumpRefresh (Variables|/Game/__MyContent/Blueprints/MyGameManager.MyGameManager_C|GetMyPlayer _my_game_manager))
    (if (Variables|Default|GetDisappears)
      (Actor|DestroyActor))))

(fn ConstructionScript
  (if (Variables|Default|GetDisappears)
    (Rendering|Material|SetMaterial (Variables|Default|GetCube) 0 "/Game/__MyContent/Materials/Material_GateRed.Material_GateRed")
    (else
      (Rendering|Material|SetMaterial (Variables|Default|GetCube) 0 "/Game/__MyContent/Materials/Material_GateBlue.Material_GateBlue"))))