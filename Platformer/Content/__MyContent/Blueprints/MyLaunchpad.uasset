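; Launchpad actor that launches the player upward when they enter its box trigger.
; On overlap by a player-tagged actor, it launches the game manager's player reference, plays a whoosh, enables the double-jump flag and hides a jump indicator.
; It then locks itself for a short cooldown, swapping the gate cube material from blue to red and back when ready.
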(event OnComponentBeginOverlap(Box)
  (params (OverlappedComponent :type Primitive%20Component%20Object%20Reference) (OtherActor :type Actor%20Object%20Reference) (OtherComp :type Primitive%20Component%20Object%20Reference) (OtherBodyIndex :type Integer) (bFromSweep :type Boolean) (SweepResult :type Hit%20Result%20Structure%20%28by%20ref%29))
  (if (Variables|Default|GetIs%20Ready)
    (if (Actor|ActorHasTag OtherActor "Tag_Player")
      (bind _my_game_manager (CallFunction|GetMyGameManager))
      (Character|LaunchCharacter (Variables|/Game/__MyContent/Blueprints/MyGameManager.MyGameManager_C|GetMyPlayer _my_game_manager) "0, 0,1250.000000" false false)
      (Audio|PlaySound2D "/Game/__MyContent/Audio/Whoosh2.Whoosh2" 4.0 0.75 0.0 0 0)
      (Default|SetJumpIndicators (Variables|/Game/__MyContent/Blueprints/MyGameManager.MyGameManager_C|GetMyPlayer _my_game_manager) false 1)
      (Variables|/Game/ThirdPersonBP/Blueprints/ThirdPersonCharacter.ThirdPersonCharacter_C|SetDoubleJump (Variables|/Game/__MyContent/Blueprints/MyGameManager.MyGameManager_C|GetMyPlayer _my_game_manager) true)
      (Variables|Default|SetIs%20Ready false)
      (Rendering|Material|SetMaterial (Variables|Default|GetGateCube) 0 "/Game/__MyContent/Materials/Material_GateRed.Material_GateRed")
      (Utilities|FlowControl|Delay 3.0)
      (Variables|Default|SetIs%20Ready true)
      (Rendering|Material|SetMaterial (Variables|Default|GetGateCube) 0 "/Game/__MyContent/Materials/Material_GateBlue.Material_GateBlue"))))

(event EventBeginPlay)

(event Collision|EventActorBeginOverlap
  (params (OtherActor :type Actor%20Object%20Reference)))

(event EventTick
  (params (DeltaSeconds :type Float%20%28single-precision%29)))

(fn ConstructionScript)