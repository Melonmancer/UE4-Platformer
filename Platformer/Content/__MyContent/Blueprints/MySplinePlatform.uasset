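; MySplinePlatform is a moving platform actor that travels along a spline path.
; On BeginPlay, a timeline plays from the start, and its SplineDistance track, scaled by the spline's length, picks the world location where the mesh is placed on each update, without sweeping.
; The construction script applies the StaticMesh and Material variables to the platform mesh.
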(event Custom|Platform%20Start
  (bind _spline_distance (Timeline|Motion%20Timeline PlayFromStart)
    (:Update
      (Transformation|SetWorldLocation (Variables|Default|GetPlatformMesh) (Spline|GetLocationatDistanceAlongSpline (Variables|Default|GetSpline) (* _spline_distance (Spline|GetSplineLength (Variables|Default|GetSpline))) "World") false false))))

(event EventBeginPlay
  (CallFunction|PlatformStart))

(event Collision|EventActorBeginOverlap
  (params (OtherActor :type Actor%20Object%20Reference)))

(event EventTick
  (params (DeltaSeconds :type Float%20%28single-precision%29)))

(fn ConstructionScript
  (bind _platformmesh (Variables|Default|GetPlatformMesh))
  (Components|StaticMesh|SetStaticMesh _platformmesh (Variables|Default|GetStatic%20Mesh))
  (Rendering|Material|SetMaterial _platformmesh 0 (Variables|Default|GetMaterial)))