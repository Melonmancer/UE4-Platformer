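; Game manager Blueprint that tracks the game state (Running, Win, Lose, Abandon) and switches the UI to match.
; Init creates the health and three end-screen widgets, initializes the player and enters Running.
; On a state change, SetState hides the UI, then either shows the HUD without mouse or the matching end screen with mouse.
; ResetGame only re-initializes the player, and ShowHUD ignores its input, always showing the health widget.
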(event EventBeginPlay)

(event Collision|EventActorBeginOverlap
  (params (OtherActor :type Actor%20Object%20Reference)))

(event EventTick
  (params (DeltaSeconds :type Float%20%28single-precision%29)))

(fn ConstructionScript)

(fn Init
  (CallFunction|CreateUI)
  (Default|Init (Variables|Default|GetMyPlayer))
  (CallFunction|SetState "NewEnumerator0"))

(fn SetState
  (params (New%20State :type MyGameStates%20Enum :default "NewEnumerator0"))
  (if (Utilities|Enum|NotEqual(Enum) New%20State (Variables|Default|GetCurrent%20Game%20State))
    (CallFunction|HideUI)
    (bind _output_get (Variables|Default|SetCurrent%20Game%20State New%20State))
    (switch Utilities|FlowControl|Switch|SwitchonMyGameStates _output_get
      (:NewEnumerator0
        (CallFunction|ShowMouse false)
        (CallFunction|ShowHUD true))
      (:NewEnumerator1
        (Widget|SetVisibility (Variables|Default|GetWidget%20Win) "Visible")
        (CallFunction|ShowMouse true :!label _label))
      (:NewEnumerator2
        (Widget|SetVisibility (Variables|Default|GetWidget%20Lose) "Visible")
        (goto _label))
      (:NewEnumerator3
        (Widget|SetVisibility (Variables|Default|GetWidget%20Abandon) "Visible")
        (goto _label)))))

(fn GetState
  (return (Variables|Default|GetCurrent%20Game%20State)))

(fn CreateUI
  (bind _returnvalue (UserInterface|CreateWidget "/Game/__MyContent/UI/Widget_Abandon.Widget_Abandon_C"))
  (bind _output_get (Variables|Default|SetWidget%20Abandon _returnvalue))
  (UserInterface|Viewport|AddtoViewport _output_get 0)
  (bind _returnvalue_2 (UserInterface|CreateWidget "/Game/__MyContent/UI/Widget_Lose.Widget_Lose_C"))
  (bind _output_get_2 (Variables|Default|SetWidget%20Lose _returnvalue_2))
  (UserInterface|Viewport|AddtoViewport _output_get_2 0)
  (bind _returnvalue_3 (UserInterface|CreateWidget "/Game/__MyContent/UI/Widget_Win.Widget_Win_C"))
  (bind _output_get_3 (Variables|Default|SetWidget%20Win _returnvalue_3))
  (UserInterface|Viewport|AddtoViewport _output_get_3 0)
  (bind _returnvalue_4 (UserInterface|CreateWidget "/Game/__MyContent/UI/Widget_Health.Widget_Health_C"))
  (bind _output_get_4 (Variables|Default|SetWidget%20Health _returnvalue_4))
  (UserInterface|Viewport|AddtoViewport _output_get_4 0))

(fn ResetGame
  (Default|Init (Variables|Default|GetMyPlayer)))

(fn ShowHUD
  (params (Visible :type Boolean))
  (bind _widget_health (Variables|Default|GetWidget%20Health))
  (if true
    (Widget|SetVisibility _widget_health "Visible")
    (else
      (Widget|SetVisibility _widget_health "Hidden"))))