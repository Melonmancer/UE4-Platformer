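; Checkpoint actor that records itself as the player's last checkpoint and restores their health to 100.
; An overlap of its box by an actor tagged as player triggers it once, via the game manager's player reference, then swaps two cube materials to a glowing used look.
; Manual Use applies the same effect without checks, Reset restores the unused look, and the construction script shows the used look when Used is set.
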(event OnComponentBeginOverlap(Box)
  (params (OverlappedComponent :type Primitive%20Component%20Object%20Reference) (OtherActor :type Actor%20Object%20Reference) (OtherComp :type Primitive%20Component%20Object%20Reference) (OtherBodyIndex :type Integer) (bFromSweep :type Boolean) (SweepResult :type Hit%20Result%20Structure%20%28by%20ref%29))
  (if (Actor|ActorHasTag OtherActor "Tag_Player")
    (if (not (Variables|Default|GetUsed))
      (bind _my_game_manager (CallFunction|GetMyGameManager))
      (Variables|/Game/ThirdPersonBP/Blueprints/ThirdPersonCharacter.ThirdPersonCharacter_C|SetLastCheckpoint (Variables|/Game/__MyContent/Blueprints/MyGameManager.MyGameManager_C|GetMyPlayer _my_game_manager) self)
      (Default|SetHealth (Variables|/Game/__MyContent/Blueprints/MyGameManager.MyGameManager_C|GetMyPlayer _my_game_manager) 1e+02)
      (Rendering|Material|SetMaterial (Variables|Default|GetCube) 0 "/Game/__MyContent/Materials/Material_SolidWhiteGlow.Material_SolidWhiteGlow")
      (Rendering|Material|SetMaterial (Variables|Default|GetCube1) 0 "/Game/__MyContent/Materials/Material_Invisible.Material_Invisible")
      (Variables|Default|SetUsed true))))

(event EventBeginPlay)

(event Collision|EventActorBeginOverlap
  (params (OtherActor :type Actor%20Object%20Reference)))

(event EventTick
  (params (DeltaSeconds :type Float%20%28single-precision%29)))

(fn ConstructionScript
  (if (Variables|Default|GetUsed)
    (Rendering|Material|SetMaterial (Variables|Default|GetCube) 0 "/Game/__MyContent/Materials/Material_SolidWhiteGlow.Material_SolidWhiteGlow")
    (Rendering|Material|SetMaterial (Variables|Default|GetCube1) 0 "/Game/__MyContent/Materials/Material_Invisible.Material_Invisible")))

(fn Reset
  (Variables|Default|SetUsed false)
  (Rendering|Material|SetMaterial (Variables|Default|GetCube) 0 "/Engine/BasicShapes/BasicShapeMaterial.BasicShapeMaterial")
  (Rendering|Material|SetMaterial (Variables|Default|GetCube1) 0 "/Game/__MyContent/Materials/Material_Whitetrans.Material_Whitetrans"))

(fn ManualUse
  (bind _my_game_manager (CallFunction|GetMyGameManager))
  (Variables|/Game/ThirdPersonBP/Blueprints/ThirdPersonCharacter.ThirdPersonCharacter_C|SetLastCheckpoint (Variables|/Game/__MyContent/Blueprints/MyGameManager.MyGameManager_C|GetMyPlayer _my_game_manager) self)
  (Default|SetHealth (Variables|/Game/__MyContent/Blueprints/MyGameManager.MyGameManager_C|GetMyPlayer _my_game_manager) 1e+02)
  (Rendering|Material|SetMaterial (Variables|Default|GetCube) 0 "/Game/__MyContent/Materials/Material_SolidWhiteGlow.Material_SolidWhiteGlow")
  (Rendering|Material|SetMaterial (Variables|Default|GetCube1) 0 "/Game/__MyContent/Materials/Material_Invisible.Material_Invisible")
  (Variables|Default|SetUsed true))